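; Master destructible actor that loses HP from projectile hits, breaks, then respawns in place.
; Overlaps on the Normal component with actors tagged "Projec" decrement HP; at zero, Normal, Box and Cube lose collision and hide.
; After a short delay they reappear with collision and HP reset.
; ItemToSpawn spawns only on the actor's Destroyed event, which the HP depletion path never triggers.
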(event OnComponentBeginOverlap(Normal)
  (params (OverlappedComponent :type Primitive%20Component%20Object%20Reference) (OtherActor :type Actor%20Object%20Reference) (OtherComp :type Primitive%20Component%20Object%20Reference) (OtherBodyIndex :type Integer) (bFromSweep :type Boolean) (SweepResult :type Hit%20Result%20Structure%20%28by%20ref%29))
  (bind _normal (Variables|Default|GetNormal))
  (if (Actor|ActorHasTag OtherActor "Projec")
    (bind _output_get (Variables|Default|SetHP (- (Variables|Default|GetHP) 1)))
    (if (<= _output_get 0)
      (Collision|SetCollisionEnabled _normal "NoCollision")
      (Development|SetHiddeninGame _normal true false)
      (Utilities|FlowControl|Delay 5.0)
      (Development|SetHiddeninGame _normal false false)
      (Collision|SetCollisionEnabled _normal "QueryAndPhysics")
      (Variables|Default|SetHP 10))))

(event EventBeginPlay)

(event Collision|EventActorBeginOverlap
  (params (OtherActor :type Actor%20Object%20Reference)))

(event EventTick
  (params (DeltaSeconds :type Float%20%28single-precision%29)))

(event EventDestroyed
  (Game|SpawnActorfromClass (Variables|Default|GetItemToSpawn) (Transformation|GetActorTransform) "Undefined" 0 0))

(fn ConstructionScript)