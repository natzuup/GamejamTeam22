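; Kill zone actor that handles death and respawn when a BP_ThirdPersonCharacter overlaps it.
; The overlap plays a death sound, fades the camera out and shows the WBP_Dead widget.
; After timed delays, it plays a spawn sound, removes the widget, moves the same character to the Checkpoints actor's location and fades the view back in.
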(event EventBeginPlay)

(event Collision|EventActorBeginOverlap
  (params (OtherActor :type Actor%20Object%20Reference))
  (bind _returnvalue (Game|GetPlayerCameraManager 0))
  (bind _asbp_third_person_character (Utilities|Casting|CastToBP_ThirdPersonCharacter OtherActor))
  (Audio|PlaySound2D "/Game/Sounds/Dieing/SC_Die.SC_Die" 1.0 1.0 0.0 0 0)
  (CameraFades|StartCameraFade :self _returnvalue :ToAlpha 1.0 :Duration 1.0 :bHoldWhenFinished true)
  (bind _returnvalue_2 (UserInterface|CreateWidget "/Game/UI/WBP_Dead.WBP_Dead_C"))
  (UserInterface|Viewport|AddtoViewport _returnvalue_2 0)
  (Utilities|FlowControl|Delay 3.0)
  (Audio|PlaySound2D "/Game/Sounds/SFX/Spawn.Spawn" 1.0 1.0 0.0 0 0)
  (Utilities|FlowControl|Delay 1.0)
  (Widget|RemovefromParent _returnvalue_2)
  (Transformation|SetActorLocation _asbp_third_person_character (Transformation|GetActorLocation (Variables|Default|GetCheckpoints)) false false)
  (Utilities|FlowControl|Delay 0.1)
  (CameraFades|StartCameraFade :self _returnvalue :FromAlpha 1.0 :Duration 0.5 :bHoldWhenFinished true))

(fn ConstructionScript)