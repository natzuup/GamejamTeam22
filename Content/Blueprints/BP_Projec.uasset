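; BP_Projec is an actor, apparently a projectile, that destroys objects tagged "Dest" when they overlap its Sphere component.
; On such an overlap it spawns box explosion and burst Niagara effects at the sphere's location.
; After a brief delay it stores the hit actor's transform, plays a 2D hit sound and destroys that actor, without destroying itself.
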(event OnComponentBeginOverlap(Sphere)
  (params (OverlappedComponent :type Primitive%20Component%20Object%20Reference) (OtherActor :type Actor%20Object%20Reference) (OtherComp :type Primitive%20Component%20Object%20Reference) (OtherBodyIndex :type Integer) (bFromSweep :type Boolean) (SweepResult :type Hit%20Result%20Structure%20%28by%20ref%29))
  (bind _sphere (Variables|Default|GetSphere))
  (bind _returnvalue (Transformation|GetWorldLocation _sphere))
  (bind _output_get (Variables|Default|SetHitActor OtherActor))
  (if (Actor|ActorHasTag _output_get "Dest")
    (Niagara|SpawnSystematLocation "/Game/Effects/NS_BoxExplosion.NS_BoxExplosion" _returnvalue)
    (Niagara|SpawnSystematLocation "/Game/Effects/NS_Burst.NS_Burst" _returnvalue)
    (Utilities|FlowControl|Delay 0.125)
    (Variables|Default|SetHitActorTransform (Transformation|GetActorTransform (Variables|Default|GetHitActor)))
    (Audio|PlaySound2D "/Game/Sounds/SpellSounds/SC_TwinkleSpellsHits.SC_TwinkleSpellsHits" 1.0 1.0 0.0 0 0)
    (Actor|DestroyActor (Variables|Default|GetHitActor))))

(fn ConstructionScript)