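; Base interactable actor that reacts when the third-person character overlaps it, according to its CollectableType.
; Overlap casts to BP_ThirdPersonCharacter, stores it as Player (never read here), then switches on the type enum.
; Eyes and Wings print their type and call Pickup, which only hides the actor and prints a debug message.
; Enemy Spike calls the Enemy event, which is an empty stub.
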(event Custom|Pickup
  (Rendering|SetActorHiddenInGame true)
  (Development|PrintString "PICKED UP"))

(event Custom|Enemy)

(event Collision|EventActorBeginOverlap
  (params (OtherActor :type Actor%20Object%20Reference))
  (bind _collectabletype (Variables|Default|GetCollectableType))
  (bind _returnvalue (Utilities|String|EnumtoString _collectabletype))
  (bind _asbp_third_person_character (Utilities|Casting|CastToBP_ThirdPersonCharacter OtherActor))
  (Variables|Default|SetPlayer _asbp_third_person_character)
  (switch Utilities|FlowControl|Switch|SwitchonE_Collectables (Variables|Default|GetCollectableType)
    (:NewEnumerator0
      (Development|PrintString _returnvalue)
      (CallFunction|Pickup))
    (:NewEnumerator4
      (Development|PrintString _returnvalue)
      (CallFunction|Pickup))
    (:NewEnumerator7
      (CallFunction|Enemy))))

(fn ConstructionScript)