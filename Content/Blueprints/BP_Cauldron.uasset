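; Cauldron actor that crafts the shrink potion when the third-person player overlaps it with crafting ready.
; Crafting removes the inventory widget, resets collected items and the ready flag, calls SizeMatters, sets UShrink and plays a sound.
; If the player is not ready and nothing has been crafted yet, a NotEnough hint appears for five seconds.
; Tick billboards that hint by setting its relative rotation from the camera-to-hint direction with inverted pitch.
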(event EventTick
  (params (DeltaSeconds :type Float%20%28single-precision%29))
  (bind _returnvalue (Game|GetPlayerCameraManager 0))
  (bind _notenough (Variables|Default|GetNotEnough))
  (bind _returnvalue_2 (Transformation|GetActorLocation _returnvalue))
  (bind _returnvalue_3 (Transformation|GetWorldLocation _notenough))
  (bind _returnvalue_4 (- _returnvalue_3 _returnvalue_2))
  (bind _returnvalue_5 (Math|Conversions|RotationFromXVector _returnvalue_4))
  (Transformation|SetRelativeRotation _notenough (Math|Rotator|MakeRotator (.roll _returnvalue_5) (* (.pitch _returnvalue_5) -1.0) (.yaw _returnvalue_5)) false false))

(event Collision|EventActorBeginOverlap
  (params (OtherActor :type Actor%20Object%20Reference))
  (bind _notenough (Variables|Default|GetNotEnough))
  (bind _asbp_third_person_character (Utilities|Casting|CastToBP_ThirdPersonCharacter OtherActor))
  (bind _output_get (Variables|Default|SetPlayer _asbp_third_person_character))
  (bind _output_get_2 (Variables|Default|SetInventory%20Widget (Variables|/Game/ThirdPerson/Blueprints/BP_ThirdPersonCharacter.BP_ThirdPersonCharacter_C|GetInventoryWidget _output_get)))
  (if (Variables|/Game/ThirdPerson/Blueprints/BP_ThirdPersonCharacter.BP_ThirdPersonCharacter_C|GetPotionCraftReady? _output_get)
    (Development|PrintString "Craft Items")
    (Widget|RemovefromParent _output_get_2)
    (Variables|/Game/ThirdPerson/Blueprints/BP_ThirdPersonCharacter.BP_ThirdPersonCharacter_C|SetItemsCollected _output_get 0)
    (Variables|/Game/ThirdPerson/Blueprints/BP_ThirdPersonCharacter.BP_ThirdPersonCharacter_C|SetPotionCraftReady? _output_get false)
    (Default|SizeMatters (Variables|Default|GetPlayer))
    (Variables|/Game/ThirdPerson/Blueprints/BP_ThirdPersonCharacter.BP_ThirdPersonCharacter_C|SetUShrink (Variables|Default|GetPlayer) true)
    (Variables|Default|SetIsCraftet true)
    ;[1 1 1] Need better Sound
    (Audio|PlaySoundatLocation "/Game/Sounds/SpellSounds/FireSpell_01.FireSpell_01" (Transformation|GetWorldLocation (Variables|Default|GetCauldronSFX)) "0, 0, 0" 1.0 1.0 0.0 0 0 0 0)
    (else
      ;[0.6226 0.1656 1] If not enough Items
      (if (not (Variables|Default|GetIsCraftet))
        (Development|SetHiddeninGame _notenough false false)
        (Utilities|FlowControl|Delay 5.0)
        (Development|SetHiddeninGame _notenough true false)))))

(fn ConstructionScript)